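; AI controller for guards that runs BT_Guard on the BB_Guard blackboard and loads sense and search settings from an XML file into variables.
; Sight updates set the target, line of sight and last known location, while other senses register as heard noise.
; Lost sight or noise resets the search timer.
; Each perception update also writes an aggressiveness score averaging clamped ramps of target distance and HP, both rising with their input.
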(event `self.ReceiveTick`
  (params (DeltaSeconds :type "Float (single-precision)")))

(event `self.ReceiveBeginPlay`
  (bind _blackboardcomponent (`self.UseBlackboard` "/Game/AI/BB_Guard.BB_Guard"))
  (`self.RunBehaviorTree` "/Game/AI/BT_Guard.BT_Guard")
  (bind (_outconfig _outerror _returnvalue) (`AIConfigLoaderBPLib.LoadAIConfigFromXML` "Content/Data/AIConfig.xml"))
  (if _returnvalue
    (`self.SetOutConfig` (break `AIConfigData` _outconfig) (`.LoseSightRadius` (break `AIConfigData` _outconfig)) (`.PeripheralVisionDegrees` (break `AIConfigData` _outconfig)) (`.HearingRange` (break `AIConfigData` _outconfig)) (`.SearchDurationSeconds` (break `AIConfigData` _outconfig)))
    (`BlackboardComponent.SetValueAsFloat` _blackboardcomponent "SearchTimeLeft" 0.0)
    (else
      (`KismetSystemLibrary.PrintString` _outerror true true (struct :`R` 1.0 :`G` 0.008737 :`B` 0.003485 :`A` 1.0) 3.0))))

(event `self.AIPerception.OnTargetPerceptionUpdated`
  (params (Actor :type "Actor Object Reference") (Stimulus :type "AIStimulus Structure"))
  (bind (_age _expirationage _strength _stimuluslocation _receiverlocation _tag _bsuccessfullysensed) (break `AIStimulus` Stimulus))
  (bind _returnvalue (`AIPerceptionSystem.GetSenseClassForStimulus` Stimulus))
  (if (== _returnvalue "/Script/AIModule.AISense_Sight")
    (if _bsuccessfullysensed
      (`BlackboardComponent.SetValueAsObject` (stale `self.ReceiveBeginPlay` _blackboardcomponent) "TargetActor" Actor)
      (`BlackboardComponent.SetValueAsBool` (stale `self.ReceiveBeginPlay` _blackboardcomponent) "HasLineOfSight" true)
      (`BlackboardComponent.SetValueAsVector` (stale `self.ReceiveBeginPlay` _blackboardcomponent) "LastKnownLocation" (`self.K2_GetActorLocation` Actor))
      (`BlackboardComponent.SetValueAsBool` (stale `self.ReceiveBeginPlay` _blackboardcomponent) "HeardNoise" false)
      (bind _agressiveness (`self.ComputeAgressiveness` (`self.GetDistanceToPlayer` (stale `self.ReceiveBeginPlay` _blackboardcomponent)) 0.0 0.0 (`self.HP`)))
      (`BlackboardComponent.SetValueAsFloat` (stale `self.ReceiveBeginPlay` _blackboardcomponent) "Agressiveness" _agressiveness)
      (else
        (`BlackboardComponent.SetValueAsBool` (stale `self.ReceiveBeginPlay` _blackboardcomponent) "HasLineOfSight" false)
        (`BlackboardComponent.SetValueAsFloat` (stale `self.ReceiveBeginPlay` _blackboardcomponent) "SearchTimeLeft" (`self.SearchDurationSeconds`))
        (bind _agressiveness_2 (`self.ComputeAgressiveness` (`self.GetDistanceToPlayer` (stale `self.ReceiveBeginPlay` _blackboardcomponent)) 0.0 0.0 (`self.HP`)))
        (`BlackboardComponent.SetValueAsFloat` (stale `self.ReceiveBeginPlay` _blackboardcomponent) "Agressiveness" _agressiveness_2)))
    (else
      (`BlackboardComponent.SetValueAsBool` (stale `self.ReceiveBeginPlay` _blackboardcomponent) "HeardNoise" true)
      (`BlackboardComponent.SetValueAsVector` (stale `self.ReceiveBeginPlay` _blackboardcomponent) "LastKnownLocation" _stimuluslocation)
      (`BlackboardComponent.SetValueAsFloat` (stale `self.ReceiveBeginPlay` _blackboardcomponent) "SearchTimeLeft" (`self.SearchDurationSeconds`))
      (bind _agressiveness_3 (`self.ComputeAgressiveness` (`self.GetDistanceToPlayer` (stale `self.ReceiveBeginPlay` _blackboardcomponent)) 0.0 0.0 (`self.HP`)))
      (`BlackboardComponent.SetValueAsFloat` (stale `self.ReceiveBeginPlay` _blackboardcomponent) "Agressiveness" _agressiveness_3))))

(fn `ComputeAgressiveness`
  (params (Distance :type "Float (double-precision)") (CloseMax :type "Float (double-precision)") (FarMin :type "Float (double-precision)") (HP :type "Float (double-precision)") (LowHP :type "Float (double-precision)") (HighHP :type "Float (double-precision)"))
  (returns (Agressiveness :type "Float (double-precision)"))
  (return (/ (+ (`KismetMathLibrary.FClamp` (/ (- Distance CloseMax) (- FarMin CloseMax)) 0.0 1.0) (`KismetMathLibrary.FClamp` (/ (- HP LowHP) (- HighHP LowHP)) 0.0)) 2.0)))

(fn `GetCurrentHP`
  (returns (CurrentHP :type "Float (double-precision)"))
  (return (`self.HP`)))

(fn `GetDistanceToPlayer`
  (params (Blackboard :type "BlackboardComponent Object Reference"))
  (returns (Distance :type "Float (double-precision)"))
  (bind _returnvalue (`BlackboardComponent.GetValueAsObject` Blackboard "TargetActor"))
  (`/Engine/EditorBlueprintResources/StandardMacros.IsValid` _returnvalue
    (:`Is Valid`
      (bind _ascharacter (cast `Character` _returnvalue))
      (return (`KismetMathLibrary.Vector_Distance` (`self.K2_GetActorLocation`) (`self.K2_GetActorLocation` _ascharacter))))))

(fn `SetOutConfig`
  (params (SightRadius :type "Float (double-precision)") (LoseSightRadius :type "Float (double-precision)") (PeripheralVisionDegrees :type "Float (double-precision)") (HearingRange :type "Float (double-precision)") (SearchDurationSeconds :type "Float (double-precision)"))
  (set `self.SightRadius` SightRadius)
  (set `self.LoseSightRadius` LoseSightRadius)
  (set `self.PeripheralVisionDegrees` PeripheralVisionDegrees)
  (set `self.HearingRange` HearingRange)
  (set `self.SearchDurationSeconds` SearchDurationSeconds))

(fn `UserConstructionScript`)